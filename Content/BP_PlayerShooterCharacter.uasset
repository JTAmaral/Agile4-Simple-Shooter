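; Player shooter character that carries two guns, fires the equipped one from the camera and interacts with nearby actors.
; Capsule overlaps send range messages through BP_InteractionInterface, and Interact triggers the first overlapping implementer.
; Pickups fill empty slots; when both are full, the equipped gun drops and PickUpGun recurses.
; Slot-based macros resolve equipped and stowed guns, which UpdateGunAttachments snaps to mesh sockets after pickups or switches.
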(event OnComponentBeginOverlap(CapsuleComponent)
  (params (OverlappedComponent :type Primitive%20Component%20Object%20Reference) (OtherActor :type Actor%20Object%20Reference) (OtherComp :type Primitive%20Component%20Object%20Reference) (OtherBodyIndex :type Integer) (bFromSweep :type Boolean) (SweepResult :type Hit%20Result%20Structure%20%28by%20ref%29))
  (if (Utilities|DoesObjectImplementInterface OtherActor "/Game/InteractionInterface/BP_InteractionInterface.BP_InteractionInterface_C")
    (Class|BPInteractionInterface|OnInteractionRangeEntered(Message) OtherActor self)))

(event OnComponentEndOverlap(CapsuleComponent)
  (params (OverlappedComponent :type Primitive%20Component%20Object%20Reference) (OtherActor :type Actor%20Object%20Reference) (OtherComp :type Primitive%20Component%20Object%20Reference) (OtherBodyIndex :type Integer))
  (if (Utilities|DoesObjectImplementInterface OtherActor "/Game/InteractionInterface/BP_InteractionInterface.BP_InteractionInterface_C")
    (Class|BPInteractionInterface|OnInteractionRangeExited(Message) OtherActor)))

(event EventBeginPlay
  (|CallParentFunction)
  (Audio|PlaySoundatLocation "/Game/AssetPacks/GameDevTV/VoiceOvers/Intro.Intro" (Transformation|GetActorLocation) "0, 0, 0" 1.0 1.0 0.0 0 0 0))

(event Collision|EventActorBeginOverlap
  (params (OtherActor :type Actor%20Object%20Reference))
  (|CallParentFunction OtherActor) ; This node is disabled and will not be called.\nDrag off pins to build functionality.
)

(event EventTick
  (params (DeltaSeconds :type Float%20%28single-precision%29))
  (|CallParentFunction DeltaSeconds) ; This node is disabled and will not be called.\nDrag off pins to build functionality.
)

(event Input|ActionEvents|InputActionShoot
  (params (Key :type Key%20Structure :default "None"))
  (:Pressed
    (bind _returnvalue (Utilities|EquippedGun)
      (:Is%20Valid
        (Default|Fire _returnvalue (Variables|Default|GetCamera))))))

(event Input|ActionEvents|InputActionInteract
  (params (Key :type Key%20Structure :default "None"))
  (:Pressed
    (bind _array_element (Utilities|Array|ForEachLoopwithBreak (Collision|GetOverlappingActors (Variables|Default|GetCapsuleComponent) "/Script/Engine.Actor" :!class /Script/Engine.PrimitiveComponent) :!label _label)
      (:LoopBody
        (if (Utilities|DoesObjectImplementInterface _array_element "/Game/InteractionInterface/BP_InteractionInterface.BP_InteractionInterface_C")
          (Class|BPInteractionInterface|OnInteracted(Message) _array_element self)
          (goto _label Break))))))

(event Input|ActionEvents|InputActionSwitchWeapons
  (params (Key :type Key%20Structure :default "None"))
  (:Pressed
    (switch Utilities|FlowControl|Switch|SwitchonE_GunSlot (Variables|Default|GetCurrentGunSlot)
      (:NewEnumerator0
        (Variables|Default|SetCurrentGunSlot "NewEnumerator1"))
      (:NewEnumerator1
        (Variables|Default|SetCurrentGunSlot "NewEnumerator0")))
    (Public|UpdateGunAttachments)))

(fn ConstructionScript
  (|CallParentFunction))

(fn PickUpGun
  (params (Gun :type BP%20Gun%20Object%20Reference))
  (Utilities|IsValid (Variables|Default|GetPrimaryGun)
    (:Is%20Valid
      (Utilities|IsValid (Variables|Default|GetSecondaryGun_0)
        (:Is%20Valid
          (bind _returnvalue (Utilities|EquippedGun)
            (:Is%20Valid
              (Transformation|DetachFromActor _returnvalue "KeepWorld" "KeepWorld" "KeepWorld")
              (Default|Drop _returnvalue)
              (Utilities|SetEquippedGun)
              (Public|PickUpGun Gun))))
        (:Is%20Not%20Valid
          (Variables|Default|SetSecondaryGun_0 Gun)
          (Public|UpdateGunAttachments :!label _label))))
    (:Is%20Not%20Valid
      (Variables|Default|SetPrimaryGun Gun)
      (goto _label))))

(fn UpdateGunAttachments
  (Utilities|FlowControl|Sequence
    (:then_0
      (bind _returnvalue (Utilities|EquippedGun)
        (:Is%20Valid
          (Transformation|AttachComponentToComponent _returnvalue (Variables|Character|GetMesh) "WeaponSocket" "SnapToTarget" "SnapToTarget" "SnapToTarget" true))))
    (:then_1
      (bind _returnvalue_2 (Utilities|StowedGun)
        (:Is%20Valid
          (Transformation|AttachComponentToComponent _returnvalue_2 (Variables|Character|GetMesh) "StowedWeaponSocket" "SnapToTarget" "SnapToTarget" "SnapToTarget" true))))))