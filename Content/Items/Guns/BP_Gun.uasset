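; BP_Gun is a gun pickup that the player can interact with, equip, drop and fire.
; SetGunState switches between Dropped, with physics and an overlap sphere active, and Equipped, with both disabled and the mesh transform reset.
; Interaction hands the gun to the player character.
; Fire spawns a BP_Laser at the ammo socket, aimed at a distant point along the camera's forward vector, plus muzzle flash and sound.
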(event EventBeginPlay
  (Private|SetGunState "NewEnumerator0"))

(event EventOnInteracted
  (params (PlayerCharacter :type BP%20Player%20Shooter%20Character%20Object%20Reference))
  (Default|PickUpGun PlayerCharacter self)
  (Private|SetGunState "NewEnumerator1"))

(fn ConstructionScript
  (|CallParentFunction))

(fn GetInteractionText
  (return "Pick Up"))

(fn GetInteractionTextAttach
  (return (Variables|Default|GetSkeletalMesh)))

(fn SetGunState
  (params (GunState :type E_GunState%20Enum :default "NewEnumerator0"))
  (bind _skeletalmesh (Variables|Default|GetSkeletalMesh))
  (bind _skeletalmesh_2 (Variables|Default|GetSkeletalMesh))
  (bind _output_get (Variables|Private|SetNewGunState GunState))
  (switch Utilities|FlowControl|Switch|SwitchonE_GunState _output_get
    (:NewEnumerator0
      (Collision|SetCollisionProfileName (Variables|Default|GetSphere) "OverlapAllDynamic" true :!class /Script/Engine.PrimitiveComponent)
      (Physics|SetSimulatePhysics _skeletalmesh_2 true)
      (Collision|SetCollisionProfileName _skeletalmesh_2 "DroppedGun" true :!class /Script/Engine.PrimitiveComponent))
    (:NewEnumerator1
      (Collision|SetCollisionProfileName (Variables|Default|GetSphere) "NoCollision" true :!class /Script/Engine.PrimitiveComponent)
      (Physics|SetSimulatePhysics _skeletalmesh false)
      (Collision|SetCollisionProfileName _skeletalmesh "NoCollision" true :!class /Script/Engine.PrimitiveComponent)
      (Transformation|ResetRelativeTransform (Variables|Default|GetSkeletalMesh)))))

(fn Drop
  (Private|SetGunState "NewEnumerator0"))

(fn Fire
  (params (PlayerCamera :type Camera%20Component%20Object%20Reference))
  (bind _skeletalmesh (Variables|Default|GetSkeletalMesh))
  (bind _returnvalue (Transformation|GetSocketLocation _skeletalmesh "AmmoSocket"))
  (Game|SpawnActorfromClass "/Game/Items/Ammo/BP_Laser.BP_Laser_C" (Math|Transform|MakeTransform _returnvalue "0, 0, 0" "1,1,1") "Undefined" 0 (* (Math|Vector|Normalize (- (+ (Transformation|GetWorldLocation PlayerCamera) (* (Math|Vector|GetForwardVector PlayerCamera) 10000)) _returnvalue)) 1e+04) 0)
  (Effects|SpawnEmitteratLocation "/Game/AssetPacks/ShooterGame/Effects/ParticleSystems/Weapons/AssaultRifle/Impacts/P_AssaultRifle_IH.P_AssaultRifle_IH" (Transformation|GetSocketLocation (Variables|Default|GetSkeletalMesh) "MuzzleFlashSocket"))
  (Audio|SpawnSoundAttached "/Game/SFX/A_RifleShot_Cue.A_RifleShot_Cue" (Variables|Default|GetSkeletalMesh) "None" "0, 0, 0" "0, 0, 0" "KeepRelativeOffset" false 1.0 1.0 0.0 0 0))