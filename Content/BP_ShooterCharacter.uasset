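; BP_ShooterCharacter is a shooter character Blueprint that tracks its own EnemyHealth and handles damage and death.
; Each AnyDamage event subtracts a fixed amount from EnemyHealth, regardless of the damage dealt.
; At zero or below, it detaches from its controller and disables capsule collision.
; A backward death animation node exists but is unconnected, so it never plays.
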(event EventBeginPlay)

(event Collision|EventActorBeginOverlap
  (params (OtherActor :type Actor%20Object%20Reference)))

(event EventTick
  (params (DeltaSeconds :type Float%20%28single-precision%29)))

(event Game|Damage|EventAnyDamage
  (params (Damage :type Float%20%28single-precision%29) (DamageType :type Damage%20Type%20Object%20Reference) (InstigatedBy :type Controller%20Object%20Reference) (DamageCauser :type Actor%20Object%20Reference))
  (Variables|Components|SetEnemyHealth (- (Variables|Components|GetEnemyHealth) 1e+01))
  (if (<= (Variables|Components|GetEnemyHealth) 0.0)
    (Class|Pawn|DetachfromControllerPendingDestroy self)
    (Collision|SetCollisionEnabled (Variables|Default|GetCapsuleComponent) "NoCollision")))

(fn ConstructionScript)